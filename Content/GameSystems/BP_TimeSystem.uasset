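; BP_TimeSystem keeps the in-game date and time, advancing it every tick at a scaled rate.
; Registered listeners receive the new time and delta on each update, plus a day-change callback when DayHasChanged reports one.
; A newly added listener gets the current time immediately.
; Skip functions jump by a timespan, to a given time or to the next calendar day's morning, then notify listeners.
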(event Custom|UpdateTimeListeners
  (params (DT :type Timespan%20Structure))
  (bind (_returnvalue _new_day) (Utilities|DayHasChanged DT))
  (for _array_element (Variables|Default|GetTimeListeners)
    (Default|OnTimeUpdated _array_element (Variables|Default|GetInGameTIme) DT)
    (if _returnvalue
      (Default|OnDayChanged _array_element _new_day (Variables|Default|GetInGameTIme)))))

(event EventTick
  (params (DeltaSeconds :type Float%20%28single-precision%29))
  (bind _ingametimeperdt (Variables|Default|GetInGameTimePerDT))
  (bind _returnvalue (* _ingametimeperdt DeltaSeconds))
  (Variables|Default|SetInGameTIme (+ (Variables|Default|GetInGameTIme) _returnvalue))
  (CallFunction|UpdateTimeListeners _returnvalue))

(fn GetinGameTime
  (return (Variables|Default|GetInGameTIme)))

(fn AddTimeListener
  (params (NewItem :type BI%20Time%20Listener%20Interface%20%28by%20ref%29))
  (Utilities|Array|AddUnique (Variables|Default|GetTimeListeners) NewItem)
  (Default|OnTimeUpdated NewItem (Variables|Default|GetInGameTIme)))

(fn SkipTime
  (params (Timespan :type Timespan%20Structure))
  (Variables|Default|SetInGameTIme (+ (Variables|Default|GetInGameTIme) Timespan))
  (CallFunction|UpdateTimeListeners Timespan))

(fn SkipTimeUntil
  (params (NewTime :type Date%20Time%20Structure))
  (Utilities|FlowControl|Sequence
    (:then_0
      (bind _output_get (LocalVariables|SetDT (- NewTime (Variables|Default|GetInGameTIme))))
      (Development|PrintString (Utilities|String|ToString(Float) (Class|KismetMathLibrary|GetTotalMilliseconds _output_get))))
    (:then_1
      (Variables|Default|SetInGameTIme NewTime)
      (CallFunction|UpdateTimeListeners (LocalVariables|GetDT)))))

(fn SkipTimeUntilNextMorning
  (bind _returnvalue (Math|Timespan|MakeTimespan 1))
  (bind _ingametime (Variables|Default|GetInGameTIme))
  (bind _returnvalue_2 (+ _ingametime _returnvalue))
  (bind (_year _month _day) (Math|DateTime|BreakDateTime _returnvalue_2))
  (CallFunction|SkipTimeUntil (Math|DateTime|MakeDateTime _year _month _day 7 30)))