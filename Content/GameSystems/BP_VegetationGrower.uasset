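; Vegetation actor that grows fruit over in-game time until it is ready to harvest.
; A DataTable row sets the fruit mesh, billboard icon and grow time, applied to the children of VegetationParent.
; As a listener of the top-down controller's BP_TimeSystem, it updates randomly varied fruit scales and a progress bar, then shows a light and harvest text.
; StartGrowing restarts the cycle and Harvest hides the vegetation.
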(event Custom|Start%20Growing
  (Variables|Default|SetTime%20Fully%20Grown (+ (Variables|/Game/GameSystems/BP_TimeSystem.BP_TimeSystem_C|GetInGameTIme (Variables|Default|GetTimeSystem)) (Variables|Default|GetTime%20To%20Grow)))
  (Utilities|SetVegetationVisibility true
    (:Completed
      (CallFunction|RandomizeFruitScales)
      (CallFunction|SetBaseScale 0.0)
      (Rendering|SetVisibility (Variables|Default|GetPointLight) false false)
      (Rendering|SetVisibility (Variables|Default|GetHarvestText) false false))))

(event Custom|Harvest
  (Rendering|SetVisibility (Variables|Default|GetPointLight) false false)
  (Rendering|SetVisibility (Variables|Default|GetHarvestText) false false)
  (Utilities|SetVegetationVisibility false))

(event EventBeginPlay
  (CallFunction|Init)
  (|SetTimeDependencies_2_2))

(event EventOnTimeUpdated
  (params (NewTime :type Date%20Time%20Structure) (DT :type Timespan%20Structure))
  (if (CallFunction|VegetationHasGrown)
    (Rendering|SetVisibility (Variables|Default|GetPointLight) true false)
    (Rendering|SetVisibility (Variables|Default|GetHarvestText) true false)
    (Widget|SetVisibility (UserInterface|GetWidget (Variables|Default|GetProgressBarWidgetComponent)) "Hidden")
    (else
      (Utilities|FlowControl|Sequence
        (:then_0
          (CallFunction|SetBaseScale (|CalcFruitscale_2 NewTime)))
        (:then_1
          (Default|SetPercentBasedonTimeLeft (Variables|Default|GetProgressBarWidgetComponent) (Variables|Default|GetTime%20Fully%20Grown) NewTime (Variables|Default|GetTime%20To%20Grow)))))))

(fn VegetationHasGrown
  (return (and (< (Variables|Default|GetTime%20Fully%20Grown) (Default|GetinGameTime (Variables|Default|GetTimeSystem))) (CallFunction|VegetationIsVisible))))

(fn RandomizeFruitScales
  (bind _variance (Variables|Default|GetVariance))
  (for _index (range 0 (Utilities|Array|Length (Variables|Default|GetFruitMeshes)))
    (Utilities|Array|SetArrayElem (Variables|Default|GetFruitScales) _index (Math|Random|RandomFloatinRange (- 1.0 _variance) (+ 1.0 _variance)) true)))

(fn InitFruits
  (params (RowName :type Name%20%28by%20ref%29))
  (bind _returnvalue (Utilities|GetDataTableRow (Variables|Default|GetData%20Table) RowName)
    (:then
      (Utilities|SetVegetationVisibility true
        (:Completed
          (Rendering|Components|Sprite|SetSprite (Variables|Default|GetBillboard) (.Texture (Utilities|Struct|BreakFPlantableStruct _returnvalue)))
          (for _array_element (Variables|Default|GetFruitMeshes)
            (bind _asstatic_mesh_component (Utilities|Casting|CastToStaticMeshComponent _array_element))
            (Components|StaticMesh|SetStaticMesh _asstatic_mesh_component (.Mesh (Utilities|Struct|BreakFPlantableStruct _returnvalue)))
            (Transformation|SetWorldScale3D _asstatic_mesh_component "0, 0, 0")
            (Variables|Default|SetTime%20To%20Grow (.TimeToGrow (Utilities|Struct|BreakFPlantableStruct _returnvalue))))
          (return))))
    (:RowNotFound
      (Utilities|SetVegetationVisibility false
        (:Completed
          (return))))))

(fn Init
  (Utilities|FlowControl|Sequence
    (:then_0
      (|SetFruitMeshes_2))
    (:then_1
      (CallFunction|InitFruits (Variables|Default|GetVegetation%20Name))
      (CallFunction|SetBaseScale (Variables|Default|GetMax%20Base%20scale)))))

(fn VegetationIsVisible
  (return (Rendering|IsVisible (Utilities|Array|Get(acopy) (Variables|Default|GetFruitMeshes)))))

(fn SetBaseScale
  (params (InputPin :type Float%20%28double-precision%29))
  (for (_array_element _array_index) (Variables|Default|GetFruitMeshes)
    (Transformation|SetWorldScale3D _array_element (Math|Vector|MakeVector (* (Utilities|Array|Get(acopy) (Variables|Default|GetFruitScales) _array_index) InputPin) (* (Utilities|Array|Get(acopy) (Variables|Default|GetFruitScales) _array_index) InputPin) (* (Utilities|Array|Get(acopy) (Variables|Default|GetFruitScales) _array_index) InputPin))))
  (return))

(fn SetTimeFullyGrownbyPercentageOfTimeLeft
  (params (Percentage :type Float%20%28double-precision%29))
  (bind _timesystem (Variables|Default|GetTimeSystem))
  (bind _ingametime (Default|GetinGameTime _timesystem))
  (Variables|Default|SetTime%20Fully%20Grown (+ _ingametime (* (- (Variables|Default|GetTime%20Fully%20Grown) _ingametime) Percentage))))

(fn VegetationIsGrowing
  (return (and (CallFunction|VegetationIsVisible) (not (CallFunction|VegetationHasGrown)))))