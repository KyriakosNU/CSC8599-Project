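; BP_SoundManager plays 2D sound effects for eating, planting, harvesting, tilting, watering and footsteps.
; Each action has its own function that plays a one-shot sound at a shared VolumeMultiplier.
; Footsteps instead use a persistent audio component, spawned on BeginPlay with auto-destroy off and stopped at once, which start and stop functions then control.
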(event EventBeginPlay
  (CallFunction|InitFootstepSound))

(fn PlayEatingSound
  (Audio|PlaySound2D (LocalVariables|GetEatingSound) (Variables|Default|GetVolume%20Multiplier) 1.0 0.0 0 0))

(fn PlayPlantingSound
  (Audio|PlaySound2D (LocalVariables|GetPlantingSound) (Variables|Default|GetVolume%20Multiplier) 1.0 0.0 0 0))

(fn PlayHarvestingSound
  (Audio|PlaySound2D (LocalVariables|GetHarvesting%20Sound) (Variables|Default|GetVolume%20Multiplier) 1.0 0.0 0 0))

(fn StartFootstepSound
  (Audio|Components|Audio|Play (Variables|Default|GetFootStepSound%20Audio%20Component) 0.0))

(fn StopFootstepSound
  (bind _footstepsound_audio_component (Variables|Default|GetFootStepSound%20Audio%20Component))
  (if (Audio|Components|Audio|IsPlaying _footstepsound_audio_component)
    (Audio|Components|Audio|Stop _footstepsound_audio_component)))

(fn InitFootstepSound
  (bind _returnvalue (Audio|SpawnSound2D (LocalVariables|GetFootstep%20Sound%20) (Variables|Default|GetVolume%20Multiplier) 1.0 0.0 0 false false))
  (Variables|Default|SetFootStepSound%20Audio%20Component _returnvalue)
  (CallFunction|StopFootstepSound))

(fn PlayTiltingSound
  (Audio|PlaySound2D "/Game/GameSystems/Data/SoundSystemFiles/SC_Tilting.SC_Tilting" (Variables|Default|GetVolume%20Multiplier) 1.0 0.0 0 0))

(fn PlayWateringSound
  (Audio|PlaySound2D (LocalVariables|GetWateringSound) (Variables|Default|GetVolume%20Multiplier) 1.0 0.0 0 0))