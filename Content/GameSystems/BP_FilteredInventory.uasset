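; BP_FilteredInventory is an inventory subclass that only holds items whose keys are on an allowed list.
; It overrides the holdable-amount query, returning zero for disallowed keys and deferring to the parent's calculation otherwise.
; The allowed check sets the key's StackID to zero before lookup, so every stack of an item matches.
; A setter clears and rebuilds the allowed list from supplied names.
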(fn GetAmmountThatCanbeHeld
  (params (Key :type F%20Inventory%20Map%20Key%20Struct%20Structure) (Ammount%20 :type Integer))
  (bind _returnvalue (CallFunction|IsAllowedInventoryKey Key))
  (if _returnvalue
    (bind _returnvalue_2 (|CallParentFunction Key Ammount%20))
    (return _returnvalue_2)
    (else
      (return 0))))

(fn SetAllowedInventoryKeysbyNames
  (params (NewParam :type Array%20of%20Names))
  (Utilities|Array|Clear (Variables|Default|GetAllowedInventoryKeys))
  (for _array_element NewParam
    (Utilities|Array|Add (Variables|Default|GetAllowedInventoryKeys) (Utilities|Struct|MakeFInventoryMapKeyStruct _array_element))))

(fn IsAllowedInventoryKey
  (params (Key :type F%20Inventory%20Map%20Key%20Struct%20Structure))
  (bind _structout (Utilities|Struct|SetmembersinFInventoryMapKeyStruct Key))
  (return (Utilities|Array|ContainsItem (Variables|Default|GetAllowedInventoryKeys) _structout)))