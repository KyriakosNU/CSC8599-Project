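; Day/night cycle component that drives a SunSky from the game's time system.
; On BeginPlay it registers as a time listener with the BP_TimeSystem component on the BP_TopDownController.
; Time updates convert hour, minute and second into a fractional solar time and refresh the sun.
; Day changes set the SunSky month and day without refreshing the sun themselves.
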(event EventBeginPlay
  (bind _returnvalue (Actor|GetActorOfClass "/Game/TopDown/Blueprints/BP_TopDownController.BP_TopDownController_C"))
  (Default|AddTimeListener (Actor|GetComponentbyClass _returnvalue "/Game/GameSystems/BP_TimeSystem.BP_TimeSystem_C") self))

(event EventOnTimeUpdated
  (params (NewTime :type Date%20Time%20Structure) (DT :type Timespan%20Structure))
  (bind (_year _month _day _hour _minute _second) (Math|DateTime|BreakDateTime NewTime))
  (bind _sunsky (Variables|Default|GetSunSky))
  (Variables|/SunPosition/SunSky.SunSky_C|SetSolarTime _sunsky (+ _hour (Math|Float|MapRangeClamped (+ _minute (/ (Math|Conversions|ToFloat(Integer) _second) 6e+01)) 0.0 6e+01 0.0 0.99)))
  (Default|UpdateSun _sunsky))

(event EventOnDayChanged
  (params (NewDay :type Integer) (New%20Date :type Date%20Time%20Structure))
  (bind (_year _month _day) (Math|DateTime|BreakDateTime New%20Date))
  (bind _sunsky (Variables|Default|GetSunSky))
  (Variables|/SunPosition/SunSky.SunSky_C|SetMonth _sunsky _month)
  (Variables|/SunPosition/SunSky.SunSky_C|SetDay _sunsky _day))