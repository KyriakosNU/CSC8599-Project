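; Picks a weighted random item and amount from a loot pool Data Table passed in by the caller.
; GetTotalWeightedSumFromDataTable adds up every row's Probability to set the upper bound of a roll drawn from a random stream, with a lower bound of 1.
; GetNextItemFromDataTable then walks the rows, accumulating Probability until it reaches the roll, and returns that row's Item and Ammount.
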(fn GetNextItemfromDataTable
  (params (NewParam :type Data%20Table%20Object%20Reference))
  (Utilities|FlowControl|Sequence
    (:then_0
      (LocalVariables|SetRandomValue (Math|Random|RandomFloatinRangefromStream (Variables|Default|GetStream) 1.0 (CallFunction|GetTotalWeightedSumfromDataTable NewParam))))
    (:then_1
      (bind _outrownames (DataTable|GetDataTableRowNames NewParam))
      (for _array_element _outrownames
        (bind _returnvalue (Utilities|GetDataTableRow NewParam _array_element)
          (:then
            (bind _output_get (LocalVariables|SetTotalSum (+ (.Probability (Utilities|Struct|BreakFItemProbabilityStruct _returnvalue)) (LocalVariables|GetTotalSum))))
            (if (>= _output_get (LocalVariables|GetRandomValue))
              (return (.Item (Utilities|Struct|BreakFItemProbabilityStruct _returnvalue)) (.Ammount (Utilities|Struct|BreakFItemProbabilityStruct _returnvalue))))))))))

(fn GetTotalWeightedSumfromDataTable
  (params (NewParam :type Data%20Table%20Object%20Reference))
  (bind _outrownames (DataTable|GetDataTableRowNames NewParam))
  (for _array_element _outrownames
    (bind _returnvalue (Utilities|GetDataTableRow NewParam _array_element)
      (:then
        (LocalVariables|SetOutSum (+ (.Probability (Utilities|Struct|BreakFItemProbabilityStruct _returnvalue)) (LocalVariables|GetOutSum))))))
  (return (LocalVariables|GetOutSum)))