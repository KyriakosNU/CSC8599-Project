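; Tracks the player's currency, environmental friendliness and hunger, and handles buying, eating and recycling items.
; As a time listener it applies per-minute rates, plus a separate daily delta on day change.
; Item actions look up data tables, update inventories and resources, with eating also scaling by expiry, adding leftovers and playing sound.
; Registered listeners are notified after time ticks, item actions and direct sets, but not day changes.
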(event Custom|Init
  (params (TimeSystem :type BP%20Time%20System%20Object%20Reference) (SoundManager :type BP%20Sound%20Manager%20Object%20Reference))
  (bind _output_get (Variables|Default|SetTimeSystem TimeSystem))
  (Default|AddPerTickTimeListener _output_get self)
  (Variables|Default|SetSoundManager SoundManager))

(event Custom|On%20Resources%20changed
  (bind _array_element (Utilities|ForEachResourcesListener)
    (:LoopBody
      (Default|OnResourcesChanged _array_element (Variables|Default|GetPlayerResources)))))

(event EventOnTimeUpdated
  (params (NewTime :type Date%20Time%20Structure) (DT :type Timespan%20Structure))
  (Variables|Default|SetPlayerResources (Utilities|AddResourcesStruct (Utilities|MultResourcesStruct (Variables|Default|GetPlayerResourcesPerMinutes) (Math|Timespan|GetTotalMinutes DT)) (Variables|Default|GetPlayerResources)))
  (CallFunction|OnResourcesChanged))

(event EventOnDayChanged
  (params (NewDay :type Integer) (New%20Date :type Date%20Time%20Structure))
  (Variables|Default|SetPlayerResources (Utilities|AddResourcesStruct (Variables|Default|GetPlayerResources) (Variables|Default|GetResourcesPerDay))))

(fn MakePlayerResourcesStruct
  (params (Currency :type Float%20%28double-precision%29) (Time :type Timespan%20Structure) (EnviromentalFriendliness :type Float%20%28double-precision%29) (Hunger :type Float%20%28double-precision%29))
  (return (Utilities|Struct|MakeFPlayerResourcesStruct Currency Time EnviromentalFriendliness Hunger)))

(fn BuyItem
  (params (Inventory :type BP%20Inventory%20System%20Object%20Reference) (Key :type F%20Inventory%20Map%20Key%20Struct%20Structure%20%28by%20ref%29) (Ammount :type Integer))
  (bind _returnvalue (Utilities|GetDataTableRow "/Game/GameSystems/Data/InventorySystemDataTables/CDT_Items.CDT_Items" (.ItemName (Utilities|Struct|BreakFInventoryMapKeyStruct Key)))
    (:then
      (bind _remainder (|PlayerHasenoughcurrencytobuyitem _returnvalue Ammount)
        (:true
          (Utilities|FlowControl|Sequence
            (:then_0
              (Default|TransferItem(s)toOtherInventory Inventory Key Ammount))
            (:then_1
              (Utilities|Struct|SetmembersinFPlayerResourcesStruct (Variables|Default|GetPlayerResources) _remainder (|GetnewenviromentalFriendliness _returnvalue))
              (CallFunction|OnResourcesChanged))))))))

(fn EatFood
  (params (Inventory :type BP%20Inventory%20System%20Object%20Reference) (Key :type F%20Inventory%20Map%20Key%20Struct%20Structure%20%28by%20ref%29))
  (bind (_itemname _daystoexpire) (Utilities|Struct|BreakFInventoryMapKeyStruct Key))
  (if (< (Utilities|Struct|BreakFPlayerResourcesStruct (Variables|Default|GetPlayerResources)) 99.5)
    (bind _returnvalue (Utilities|GetDataTableRow "/Game/GameSystems/Data/InventorySystemDataTables/DT_ItemEdibleFood.DT_ItemEdibleFood" _itemname)
      (:then
        (Utilities|FlowControl|Sequence
          (:then_0
            (Default|RemoveItem(s)fromInventory Inventory Key 1))
          (:then_1
            (|Addleftoversifneeded Inventory Key))
          (:then_2
            (Utilities|Struct|SetmembersinFPlayerResourcesStruct (Variables|Default|GetPlayerResources) (* (Math|Integer|Min(Integer) _daystoexpire 1) (|GetUpdatedHungerValue _returnvalue)))
            (CallFunction|OnResourcesChanged))
          (:then_3
            (Default|PlayEatingSound (Variables|Default|GetSoundManager))))))))

(fn IsIteminDataTable
  (params (FInventoryMapKeyStruct :type F%20Inventory%20Map%20Key%20Struct%20Structure%20%28by%20ref%29) (DataTable :type Data%20Table%20Object%20Reference))
  (bind _returnvalue (Utilities|GetDataTableRow DataTable (.ItemName (Utilities|Struct|BreakFInventoryMapKeyStruct FInventoryMapKeyStruct)))
    (:then
      (return true _returnvalue))
    (:RowNotFound
      (return false ""))))

(fn AddResourcesListener
  (params (NewItem :type BI%20Resources%20Listener%20Interface%20%28by%20ref%29))
  (Utilities|Array|AddUnique (Variables|Default|GetResourcesListeners) NewItem)
  (Default|OnResourcesChanged NewItem (Variables|Default|GetPlayerResources)))

(fn RecycleItem
  (params (Inventory :type BP%20Inventory%20System%20Object%20Reference%20%28by%20ref%29))
  (bind _playerresources (Variables|Default|GetPlayerResources))
  (Utilities|FlowControl|Sequence
    (:then_0
      (bind _total_benefit (|CalcTotalbenefit Inventory)
        (:out%20
          (Utilities|Struct|SetmembersinFPlayerResourcesStruct _playerresources (+ _total_benefit (Utilities|Struct|BreakFPlayerResourcesStruct _playerresources)))
          (CallFunction|OnResourcesChanged))))
    (:then_1
      (Default|ClearItems Inventory))))

(fn SetPlayerResources
  (params (PlayerResources :type F%20Player%20Resources%20Struct%20Structure))
  (Variables|Default|SetPlayerResources PlayerResources)
  (CallFunction|OnResourcesChanged))