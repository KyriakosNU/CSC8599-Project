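; Inventory component that stores items as stacks in a map keyed by item name, stack ID and container.
; Adds and removals work on each item's highest stack ID, spilling or borrowing one stack, within stack limits from a data table or singleton flag.
; It also transfers items with a linked inventory, converts items and opens container items.
; Listeners are notified of changes, opening and closing through looped calls.
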(event Custom|InventoryClosed
  (bind _array_element (Utilities|ForEachInventoryListener)
    (:LoopBody
      (Default|OnInventoryClosed _array_element))))

(event Custom|Inventory%20changed
  (bind _array_element (Utilities|ForEachInventoryListener)
    (:LoopBody
      (Default|OnInventoryChange _array_element))))

(event Custom|RemovedItems
  (params (MapKey :type F%20Inventory%20Map%20Key%20Struct%20Structure) (Ammount :type Integer))
  (bind _array_element (Utilities|ForEachInventoryListener)
    (:LoopBody
      (Default|OnInventoryAddedItem(s) _array_element MapKey Ammount))))

(event Custom|InventoryOpened
  (bind _array_element (Utilities|ForEachInventoryListener)
    (:LoopBody
      (Default|OnInvenoryOpened _array_element))))

(event Custom|AddedItem%28s%29
  (params (MapKey :type F%20Inventory%20Map%20Key%20Struct%20Structure) (Ammount :type Integer))
  (bind _array_element (Utilities|ForEachInventoryListener)
    (:LoopBody
      (Default|OnInventoryAddedItem(s) _array_element MapKey Ammount))))

(fn PrintItem(s)inInventory
  (params (InDuration :type Float%20%28single-precision%29))
  (LocalVariables|SetDuration InDuration)
  (Development|PrintString (Utilities|String|Append "Inventory component in " (Utilities|GetDisplayName (Components|GetOwner)) " has " (Utilities|String|ToString(Integer) (Variables|Default|GetTotalStacks)) " Items : ") true true "(R=0.000000,G=0.660000,B=1.000000,A=1.000000)" (LocalVariables|GetDuration) "Inv")
  (bind _keys (Utilities|Map|Keys (Variables|Default|GetItemsContained)))
  (for (_array_element _array_index) _keys
    (Development|PrintString (Utilities|String|Append "Slot " (Utilities|String|ToString(Integer) _array_index) " has " (Utilities|String|ToString(Name) (.ItemName (Utilities|Struct|BreakFInventoryMapKeyStruct _array_element))) " x " (Utilities|String|ToString(Integer) (.Value (Utilities|Map|Find (Variables|Default|GetItemsContained) _array_element))) " in stack " (Utilities|String|ToString(Integer) (.StackID (Utilities|Struct|BreakFInventoryMapKeyStruct _array_element)))) true true "(R=0.000000,G=0.660000,B=1.000000,A=1.000000)" (LocalVariables|GetDuration) (Utilities|String|StringToName (Utilities|String|ToString(Integer) _array_index)))))

(fn AddItem(S)toInventory
  (params (Key :type F%20Inventory%20Map%20Key%20Struct%20Structure) (Ammount :type Integer))
  (bind _total_ammount (LocalVariables|GetTotal%20Ammount))
  (bind _maxstack (LocalVariables|GetMaxStack))
  (bind _returnvalue (- _total_ammount _maxstack))
  (Utilities|FlowControl|Sequence
    (:then_0
      (|Initvariables Key Ammount))
    (:then_1
      (|AddtoLaststack_2))
    (:then_2
      (|Ifcanholdanotherstack_2 _returnvalue
        (:true
          (|AddNewstack_2 _returnvalue))))
    (:then_3
      (CallFunction|AddedItem(s) Key Ammount)
      (CallFunction|InventoryChanged))))

(fn RemoveItem(s)fromInventory
  (params (Key :type F%20Inventory%20Map%20Key%20Struct%20Structure%20%28by%20ref%29) (Ammount :type Integer))
  (bind (_key _stackid _ammount) (GetFunctions|GetLastStack Key))
  (LocalVariables|Set:astStackIDKey _key)
  (LocalVariables|SetLastStackID _stackid)
  (bind _output_get (LocalVariables|SetRemainder (- _ammount Ammount)))
  (Math|Integer|CompareInt _output_get
    (:>
      (Utilities|Map|Add (Variables|Default|GetItemsContained) (LocalVariables|Get:astStackIDKey) (LocalVariables|GetRemainder)))
    (:==
      (Utilities|Map|Remove (Variables|Default|GetItemsContained) (LocalVariables|Get:astStackIDKey) :!label _label)
      (Math|Integer|DecrementInt (Variables|Default|GetTotalStacks)
        (:%20%20
          _)))
    (:<
      (|Updatesecondtolaststack)
      (goto _label)))
  (CallFunction|InventoryChanged))

(fn TransferItem(s)toOtherInventory
  (params (Key :type F%20Inventory%20Map%20Key%20Struct%20Structure%20%28by%20ref%29) (Ammount :type Integer))
  (bind _otherinventory (Variables|Default|GetOtherInventory))
  (Utilities|IsValid _otherinventory
    (:Is%20Valid
      (bind _returnvalue (GetFunctions|GetAmmountThatCanbeHeld _otherinventory Key Ammount))
      (if (> _returnvalue 0)
        (ItemStateChange|AddItem(S)toInventory (Variables|Default|GetOtherInventory) Key _returnvalue)
        (ItemStateChange|RemoveItem(s)fromInventory Key _returnvalue)))))

(fn TransferItem(s)fromOtherInventory
  (params (Index :type Integer))
  (bind (_key _ammount) (GetFunctions|GetItem(s)InSlot Index))
  (Utilities|IsValid (Variables|Default|GetOtherInventory)
    (:Is%20Valid
      (ItemStateChange|AddItem(S)toInventory _key _ammount)
      (ItemStateChange|RemoveItem(s)fromInventory (Variables|Default|GetOtherInventory) _key _ammount))))

(fn GetLastStack
  (params (FItemSlotStruct :type F%20Inventory%20Map%20Key%20Struct%20Structure))
  (for _index (range 0 (Variables|Default|GetMaxStackID))
    (bind _structout (Utilities|Struct|SetmembersinFInventoryMapKeyStruct FItemSlotStruct (- (Variables|Default|GetMaxStackID) _index)))
    (if (.ReturnValue (Utilities|Map|Find (Variables|Default|GetItemsContained) _structout))
      (return _structout (- (Variables|Default|GetMaxStackID) _index) (.Value (Utilities|Map|Find (Variables|Default|GetItemsContained) _structout)) true)))
  (bind _structout_2 (Utilities|Struct|SetmembersinFInventoryMapKeyStruct FItemSlotStruct))
  (return _structout_2 0 0 false))

(fn GetMaxStack
  (params (RowName :type Name))
  (if (Variables|Default|GetIsSingleton)
    (return 1)
    (else
      (bind _returnvalue (Utilities|GetDataTableRow (Variables|Default|GetItemsDataTable) RowName)
        (:then
          (return (.MaxStack (Utilities|Struct|BreakFItemStruct _returnvalue))))
        (:RowNotFound
          (return 1000))))))

(fn GetItem(s)InSlot
  (params (Slot%20Index :type Integer))
  (bind _itemscontained (Variables|Default|GetItemsContained))
  (if (<= Slot%20Index (Utilities|Map|Length (Variables|Default|GetItemsContained)))
    (bind _keys (Utilities|Map|Keys _itemscontained))
    (bind _values (Utilities|Map|Values _itemscontained))
    (return (Utilities|Array|Get(acopy) _keys Slot%20Index) (Utilities|Array|Get(acopy) _values Slot%20Index))
    (else
      (return (Utilities|Struct|MakeFInventoryMapKeyStruct "None" 0 "None") 0))))

(fn GetSlotsAmmount
  (return (Utilities|Map|Length (Variables|Default|GetItemsContained))))

(fn AddtoInventoryListeners
  (params (InventoryListeners :type BI%20Inventory%20Listener%20Interface%20%28by%20ref%29))
  (Utilities|Array|AddUnique (Variables|Default|GetInventoryListeners) InventoryListeners))

(fn GetAmmountThatCanbeHeld
  (params (Key :type F%20Inventory%20Map%20Key%20Struct%20Structure) (Ammount%20 :type Integer))
  (bind _itemname (Utilities|Struct|BreakFInventoryMapKeyStruct Key))
  (bind (_key _stackid _ammount _existing_item) (GetFunctions|GetLastStack Key))
  (bind _maxstack (GetFunctions|GetMaxStack _itemname))
  (bind _returnvalue (- _maxstack _ammount))
  (if (GetFunctions|CanHoldAnotherStack _stackid)
    (return (Math|Integer|Min(Integer) (+ _maxstack _returnvalue) Ammount%20))
    (else
      (return (* (|Existingitemorspacefornew _existing_item) (Math|Integer|Min(Integer) _returnvalue Ammount%20))))))

(fn CanHoldAnotherStack
  (params (Last%20Stack%20ID :type Integer))
  (return (and (< Last%20Stack%20ID (Variables|Default|GetMaxStackID)) (< (Variables|Default|GetTotalStacks) (Variables|Default|GetMaxTotalStacks)))))

(fn GetItemAmmountWKey
  (params (Key :type F%20Inventory%20Map%20Key%20Struct%20Structure%20%28by%20ref%29))
  (bind (_key _stackid _ammount _existing_item) (GetFunctions|GetLastStack Key))
  (if _existing_item
    (return (+ (* _stackid (GetFunctions|GetMaxStack (.ItemName (Utilities|Struct|BreakFInventoryMapKeyStruct Key)))) _ammount) true)
    (else
      (return 0 false))))

(fn ChangeItemstoOtherItems
  (params (InKey :type F%20Inventory%20Map%20Key%20Struct%20Structure) (OtherKey :type F%20Inventory%20Map%20Key%20Struct%20Structure%20%28by%20ref%29) (Ammount :type Integer))
  (ItemStateChange|RemoveItem(s)fromInventory InKey Ammount)
  (ItemStateChange|AddItem(S)toInventory OtherKey Ammount)
  (return true))

(fn OpenItem
  (params (InKey :type F%20Inventory%20Map%20Key%20Struct%20Structure) (Ammount :type Integer))
  (Utilities|FlowControl|Sequence
    (:then_0
      (ItemStateChange|AddItem(S)toInventory (Utilities|Struct|MakeFInventoryMapKeyStruct (Utilities|Struct|BreakFInventoryMapKeyStruct InKey)) Ammount))
    (:then_1
      (bind _structout (Utilities|Struct|SetmembersinFInventoryMapKeyStruct (|Copy InKey) "None"))
      (bind _succesful (ItemStateChange|ChangeItemstoOtherItems InKey _structout Ammount))
      (return _succesful))))

(fn ClearItems
  (Utilities|Map|Clear (Variables|Default|GetItemsContained))
  (CallFunction|InventoryChanged))

(fn GetItemNameCounts
  (bind _keys (Utilities|Map|Keys (Variables|Default|GetItemsContained)))
  (for _array_element _keys
    (if (not (Utilities|Map|Contains (LocalVariables|GetItem%20To%20Item%20Count%20Map) _array_element))
      (Utilities|Map|Add (LocalVariables|GetItem%20To%20Item%20Count%20Map) _array_element (.ReturnValue (GetFunctions|GetItemAmmountWKey _array_element)))))
  (return (LocalVariables|GetItem%20To%20Item%20Count%20Map)))