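; Tracks player meta stats from resource changes to signal win, loss and starvation to registered listeners.
; Each update steps win and lose counters up or down, floored at zero, based on high environmental friendliness and low Hunger respectively.
; Listeners are notified on every update while a counter exceeds its threshold.
; Starvation uses an XOR check against the Hunger threshold, so it notifies only when the state flips.
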(event EventOnResourcesChanged
  (params (New%20Resources :type F%20Player%20Resources%20Struct%20Structure) (Resources%20difference :type F%20Player%20Resources%20Struct%20Structure))
  (Utilities|FlowControl|Sequence
    (:then_0
      (CallFunction|UpdateWin/LossConditionStatistics New%20Resources 85.0 1e+01 2e+04 2e+01))
    (:then_1
      (CallFunction|UpdateOtherStatsitics New%20Resources 15.0))))

(fn TestforWin/LossConditions
  (params (Lose%20Condition%20Val%20Threshold :type Float%20%28double-precision%29) (Win%20Condition%20Val%20Threshold :type Float%20%28double-precision%29))
  (Utilities|FlowControl|Sequence
    (:then_0
      (if (> (Variables|Default|GetWin%20Condition%20Val) Win%20Condition%20Val%20Threshold)
        (bind _array_element (Utilities|ForEachMetaStatListener)
          (:LoopBody
            (Default|OnWinConditionMet _array_element))
          (:Completed
            (return)))))
    (:then_1
      (if (> (Variables|Default|GetLose%20Condition%20Val) Lose%20Condition%20Val%20Threshold)
        (bind _array_element_2 (Utilities|ForEachMetaStatListener)
          (:LoopBody
            (Default|OnLoseConditionMet _array_element_2))
          (:Completed
            (return)))))))

(fn UpdateWin/LossConditionStatistics
  (params (Player%20Resources :type F%20Player%20Resources%20Struct%20Structure) (Min%20env%20Friendliness :type Float%20%28double-precision%29) (Min%20Hunger :type Float%20%28double-precision%29) (Lose%20condition%20Val%20Threshold :type Float%20%28double-precision%29) (Win%20condition%20Val%20Threshold :type Float%20%28double-precision%29))
  (bind (_enviromentalfriendliness _hunger) (Utilities|Struct|BreakFPlayerResourcesStruct Player%20Resources))
  (Utilities|FlowControl|Sequence
    (:then_0
      (Variables|Default|SetWin%20Condition%20Val (Math|Float|Max(Float) (+ (Math|Float|SelectFloat 1.0 -1.0 (> _enviromentalfriendliness Min%20env%20Friendliness)) (Variables|Default|GetWin%20Condition%20Val)) 0.0)))
    (:then_1
      (Variables|Default|SetLose%20Condition%20Val (Math|Float|Max(Float) (+ (Math|Float|SelectFloat 1.0 -1.0 (< _hunger Min%20Hunger)) (Variables|Default|GetLose%20Condition%20Val)) 0.0)))
    (:then_2
      (CallFunction|TestforWin/LossConditions Lose%20condition%20Val%20Threshold Win%20condition%20Val%20Threshold))))

(fn AddMetaStatsListener
  (params (NewItem :type BI%20Player%20Meta%20Stats%20Listener%20Interface%20%28by%20ref%29))
  (Utilities|Array|AddUnique (Variables|Default|GetPlayer%20Meta%20Stats%20Listeners) NewItem))

(fn UpdateOtherStatsitics
  (params (Player%20Resources :type F%20Player%20Resources%20Struct%20Structure) (IsHungry%20Threshold :type Float%20%28double-precision%29))
  (if (Class|KismetMathLibrary|XORBoolean (< (Utilities|Struct|BreakFPlayerResourcesStruct Player%20Resources) IsHungry%20Threshold) (Variables|Default|GetIs%20Starving))
    (Utilities|FlowControl|Sequence
      (:then_0
        (bind _output_get (Variables|Default|SetIs%20Starving (not (Variables|Default|GetIs%20Starving)))))
      (:then_1
        (bind _array_element (Utilities|ForEachMetaStatListener)
          (:LoopBody
            (Default|OnStarvationStateChange _array_element _output_get)))))))