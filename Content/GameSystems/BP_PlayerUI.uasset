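; Player UI manager that creates and holds the game's widgets: inventories, shop, recipe chooser, mobile menu, clock, resources, confirmation, item info and pause menu.
; InitUI builds them all, registering widgets as listeners on the inventory, time and resource systems.
; Other-inventory and shop grids are bound later to whichever inventory is supplied, and all grids share one item-info panel.
; Helpers report open menus and the active item, show confirmations and toggle pause.
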(event Custom|Init%20UI
  (params (PlayerController :type Player%20Controller%20Object%20Reference) (InventorySystem :type BP%20Inventory%20System%20Object%20Reference) (Time%20System :type BP%20Time%20System%20Object%20Reference) (PlayerResources :type BP%20Player%20Resources%20Object%20Reference))
  (MobileMenuWidget|InitMobileMenuWidget PlayerController)
  (BackGroundWidget|InitBackground PlayerController InventorySystem)
  (InventoryWidget|InitInventoryGridWidget "NewEnumerator0" PlayerController InventorySystem (Variables|Default|GetPlayerInventoryWidget) PlayerResources true)
  (InventoryWidget|InitInventoryGridWidget "NewEnumerator2" PlayerController 0 (Variables|Default|GetOtherInventoryWidget) PlayerResources false)
  (BackGroundWidget|InitRecipeChooser PlayerController)
  (ShopInventoryWidget|InitShopInventoryGridWidget "NewEnumerator2" PlayerController 0 (Variables|Default|GetShopInventoryWidget) PlayerResources)
  (DateTimeWidget|InitDateTimeWidget PlayerController Time%20System)
  (ResourcesWidget|InitResourcesWidget PlayerController PlayerResources)
  (ConfirmationWdiget|InitConfirmationWidget PlayerController)
  (MoreInfoWidget|InitMoreInfoWidget PlayerController)
  (PauseMenu|InitPauseMenu PlayerController))

(fn InitInventoryGridWidget
  (params (PositionEnum :type EGridPositions%20Enum :default "NewEnumerator0") (PlayerController :type Player%20Controller%20Object%20Reference) (InventorySystem :type BP%20Inventory%20System%20Object%20Reference) (InventoryGridWidget :type W%20Inventory%20Grid%20Object%20Reference%20%28by%20ref%29) (PlayerResources :type BP%20Player%20Resources%20Object%20Reference) (IsPlayerInventory :type Boolean))
  (Utilities|FlowControl|Sequence
    (:then_0
      (bind _returnvalue (UserInterface|CreateWidget "/Game/GameSystems/Data/UIAssets/W_InventoryGrid.W_InventoryGrid_C" PlayerController 2.0 5.0 InventorySystem PositionEnum PlayerResources IsPlayerInventory (Variables|Default|GetMobile%20Menu%20Widget)))
      (|SetBy-RefVar InventoryGridWidget _returnvalue))
    (:then_1
      (Utilities|IsValid InventorySystem
        (:Is%20Valid
          (Default|AddtoInventoryListeners InventorySystem InventoryGridWidget)
          (Default|Init InventoryGridWidget))
        (:Is%20Not%20Valid
          _))
      (UserInterface|Viewport|AddtoViewport InventoryGridWidget 0))))

(fn InitDateTimeWidget
  (params (OwningPlayer :type Player%20Controller%20Object%20Reference) (Time%20System :type BP%20Time%20System%20Object%20Reference))
  (bind _returnvalue (UserInterface|CreateWidget "/Game/GameSystems/Data/UIAssets/W_DateTimeWidget.W_DateTimeWidget_C" OwningPlayer))
  (bind _output_get (Variables|Default|SetDateTimeWidget _returnvalue))
  (Default|AddPerTickTimeListener Time%20System _output_get)
  (UserInterface|Viewport|AddtoViewport _returnvalue 0))

(fn IsInventoryOpen
  (return (Math|Boolean|ORBoolean (Default|IsOpen (Variables|Default|GetPlayerInventoryWidget)) (Widget|IsVisible (Variables|Default|GetMobile%20Menu%20Widget)) (Default|IsOpen (Variables|Default|GetShopInventoryWidget)))))

(fn IsAMenuOpen
  (return (Math|Boolean|ORBoolean (Default|IsOpen (Variables|Default|GetPlayerInventoryWidget)) (Widget|IsVisible (Variables|Default|GetConfirmationWidget)) (Widget|IsVisible (Variables|Default|GetMobile%20Menu%20Widget)) (Default|IsOpen (Variables|Default|GetShopInventoryWidget)))))

(fn InitBackground
  (params (OwningPlayer :type Player%20Controller%20Object%20Reference) (InventorySystem :type BP%20Inventory%20System%20Object%20Reference))
  (bind _returnvalue (UserInterface|CreateWidget "/Game/GameSystems/Data/UIAssets/W_Background.W_Background_C" OwningPlayer))
  (bind _output_get (Variables|Default|SetBackgroundWidget _returnvalue))
  (Widget|SetVisibility _output_get "Hidden")
  (Default|AddtoInventoryListeners InventorySystem _output_get)
  (UserInterface|Viewport|AddtoViewport _output_get -20))

(fn InitResourcesWidget
  (params (OwningPlayer :type Player%20Controller%20Object%20Reference) (PlayerResources :type BP%20Player%20Resources%20Object%20Reference))
  (bind _returnvalue (UserInterface|CreateWidget "/Game/GameSystems/Data/UIAssets/W_Resources.W_Resources_C" OwningPlayer))
  (bind _output_get (Variables|Default|SetResourcesWidget _returnvalue))
  (Default|AddResourcesListener PlayerResources _output_get)
  (UserInterface|Viewport|AddtoViewport _output_get 0))

(fn SetOtherWidgetInventory
  (params (OtherInventorySystem :type BP%20Inventory%20System%20Object%20Reference))
  (bind _otherinventorywidget (Variables|Default|GetOtherInventoryWidget))
  (Variables|/Game/GameSystems/Data/UIAssets/W_InventoryGrid.W_InventoryGrid_C|SetInventorySystem _otherinventorywidget OtherInventorySystem)
  (Default|AddtoInventoryListeners OtherInventorySystem _otherinventorywidget))

(fn ResetOtherInventory
  (Default|OnInventoryClosed (Variables|Default|GetOtherInventoryWidget)))

(fn InitShopInventoryGridWidget
  (params (PositionEnum :type EGridPositions%20Enum :default "NewEnumerator0") (PlayerController :type Player%20Controller%20Object%20Reference) (InventorySystem :type BP%20Inventory%20System%20Object%20Reference) (InventoryGridWidget :type W%20Shop%20Inventory%20Object%20Reference%20%28by%20ref%29) (PlayerResources :type BP%20Player%20Resources%20Object%20Reference))
  (bind _returnvalue (UserInterface|CreateWidget "/Game/GameSystems/Data/UIAssets/W_ShopInventory.W_ShopInventory_C" PlayerController 2.0 5.0 InventorySystem PositionEnum PlayerResources (Variables|Default|GetMoreInfoWidget)))
  (|SetBy-RefVar InventoryGridWidget _returnvalue)
  (Utilities|IsValid InventorySystem
    (:Is%20Valid
      (Default|AddtoInventoryListeners InventorySystem _returnvalue)
      (Default|Init _returnvalue))
    (:Is%20Not%20Valid
      _))
  (UserInterface|Viewport|AddtoViewport _returnvalue 0))

(fn SetShopWidgetInventory
  (params (OtherInventorySystem :type BP%20Inventory%20System%20Object%20Reference) (Player%20Inventory :type BP%20Inventory%20System%20Object%20Reference) (Shop%20Inventory%20Text :type Text) (IsOnlineShopInventory :type Boolean))
  (bind _shopinventorywidget (Variables|Default|GetShopInventoryWidget))
  (Variables|/Game/GameSystems/Data/UIAssets/W_ShopInventory.W_ShopInventory_C|SetInventorySystem _shopinventorywidget OtherInventorySystem)
  (Default|AddtoInventoryListeners OtherInventorySystem _shopinventorywidget)
  (Variables|/Game/GameSystems/Data/UIAssets/W_ShopInventory.W_ShopInventory_C|SetShopInventoryText _shopinventorywidget Shop%20Inventory%20Text)
  (bind _output_get (Variables|/Game/GameSystems/Data/UIAssets/W_ShopInventory.W_ShopInventory_C|SetIsOnlineShopInventory _shopinventorywidget IsOnlineShopInventory))
  (if (not _output_get)
    (Variables|/Game/GameSystems/BP_InventorySystem.BP_InventorySystem_C|SetOtherInventory Player%20Inventory OtherInventorySystem)))

(fn ResetOtherShopInventory
  (Default|OnInventoryClosed (Variables|Default|GetShopInventoryWidget)))

(fn InitConfirmationWidget
  (params (OwningPlayer :type Player%20Controller%20Object%20Reference))
  (bind _returnvalue (UserInterface|CreateWidget "/Game/GameSystems/Data/UIAssets/W_Confirmation.W_Confirmation_C" OwningPlayer 0))
  (bind _output_get (Variables|Default|SetConfirmationWidget _returnvalue))
  (ConfirmationWdiget|ResetConfirmationWidget)
  (UserInterface|Viewport|AddtoViewport _output_get 0))

(fn SetConfirmationWidget
  (params (Main%20Text :type Text) (Sub%20Text :type Text) (OptionListener :type BI%20Option%20Listener%20Interface) (Remove%20No%20button :type Boolean))
  (bind _confirmationwidget (Variables|Default|GetConfirmationWidget))
  (Default|Init _confirmationwidget Main%20Text Sub%20Text OptionListener Remove%20No%20button)
  (Widget|SetVisibility _confirmationwidget "Visible"))

(fn ResetConfirmationWidget
  (bind _confirmationwidget (Variables|Default|GetConfirmationWidget))
  (Default|Init _confirmationwidget "" "" 0 false)
  (Widget|SetVisibility _confirmationwidget "Hidden"))

(fn InitMoreInfoWidget
  (params (OwningPlayer :type Player%20Controller%20Object%20Reference))
  (bind _returnvalue (UserInterface|CreateWidget "/Game/GameSystems/Data/UIAssets/W_MoreItemInfo.W_MoreItemInfo_C" OwningPlayer))
  (bind _output_get (Variables|Default|SetMoreInfoWidget _returnvalue))
  (Widget|SetVisibility _output_get "Hidden")
  (Variables|/Game/GameSystems/Data/UIAssets/W_InventoryGrid.W_InventoryGrid_C|SetW_MoreItemInfo (Variables|Default|GetPlayerInventoryWidget) _output_get)
  (Variables|/Game/GameSystems/Data/UIAssets/W_InventoryGrid.W_InventoryGrid_C|SetW_MoreItemInfo (Variables|Default|GetOtherInventoryWidget) _output_get)
  (Variables|/Game/GameSystems/Data/UIAssets/W_ShopInventory.W_ShopInventory_C|SetW_MoreItemInfo (Variables|Default|GetShopInventoryWidget) _output_get)
  (UserInterface|Viewport|AddtoViewport _output_get 0))

(fn GetActivePlayerItem
  (bind (_key _ammount) (Default|GetActiveItem (Variables|Default|GetPlayerInventoryWidget)))
  (return _key _ammount))

(fn InitPauseMenu
  (params (OwningPlayer :type Player%20Controller%20Object%20Reference))
  (bind _returnvalue (UserInterface|CreateWidget "/Game/GameSystems/Data/UIAssets/W_PauseMenu.W_PauseMenu_C" OwningPlayer self))
  (bind _output_get (Variables|Default|SetPauseMenuWidget _returnvalue))
  (Widget|SetVisibility _output_get "Hidden")
  (UserInterface|Viewport|AddtoViewport _output_get 5))

(fn ToggleGamePaused
  (bind _returnvalue (Game|IsGamePaused))
  (bind _returnvalue_2 (not _returnvalue))
  (bind _returnvalue_3 (select _returnvalue_2 "Visible" "Hidden"))
  (Utilities|FlowControl|Sequence
    (:then_0
      (Widget|SetVisibility (Variables|Default|GetBackgroundWidget) _returnvalue_3)
      (Widget|SetVisibility (Variables|Default|GetPauseMenuWidget) _returnvalue_3))
    (:then_1
      (Game|SetGamePaused _returnvalue_2))))

(fn InitRecipeChooser
  (params (OwningPlayer :type Player%20Controller%20Object%20Reference))
  (bind _returnvalue (UserInterface|CreateWidget "/Game/GameSystems/Data/UIAssets/W_RecipeChooser.W_RecipeChooser_C" OwningPlayer))
  (bind _output_get (Variables|Default|SetRecipeChooserWidget _returnvalue))
  (Widget|SetVisibility _output_get "Hidden")
  (UserInterface|Viewport|AddtoViewport _output_get 0))

(fn InitMobileMenuWidget
  (params (OwningPlayer :type Player%20Controller%20Object%20Reference))
  (bind _returnvalue (UserInterface|CreateWidget "/Game/GameSystems/Data/UIAssets/W_MobileMenu.W_MobileMenu_C" OwningPlayer))
  (bind _output_get (Variables|Default|SetMobile%20Menu%20Widget _returnvalue))
  (Widget|SetVisibility _output_get "Hidden")
  (UserInterface|Viewport|AddtoViewport (Variables|Default|GetMobile%20Menu%20Widget) 1))

(fn SetMobileMenuVisibility
  (params (InVisibility :type ESlateVisibility%20Enum :default "Visible"))
  (Widget|SetVisibility (Variables|Default|GetMobile%20Menu%20Widget) InVisibility))