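; BP_RecipeSystem converts inventory items into other items using one-to-one recipes from a data table.
; A shared loop macro feeds each recipe row's input and output names to the lookup and conversion logic.
; ChangeItemsWRecipies swaps the full amount of each matching item in the given inventory's "None" container, while IsValidRecipe returns an item's output name.
; The item-added event only stores its key and amount.
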(event Custom|Change%20Items%20WRecipies
  (params (InventorySystem :type BP%20Inventory%20System%20Object%20Reference))
  (bind (_initemname _outitemname) (Utilities|LoopThroughDataTableRows)
    (:then
      (if (.Exists (Default|GetItemAmmountWKey InventorySystem (Utilities|Struct|MakeFInventoryMapKeyStruct _initemname "None")))
        (Default|ChangeItemstoOtherItems InventorySystem (Utilities|Struct|MakeFInventoryMapKeyStruct _initemname "None") (Utilities|Struct|MakeFInventoryMapKeyStruct _outitemname "None") (.ReturnValue (Default|GetItemAmmountWKey InventorySystem (Utilities|Struct|MakeFInventoryMapKeyStruct _initemname "None"))))))))

(event EventOnInventoryAddedItem(s)
  (params (MapKey :type F%20Inventory%20Map%20Key%20Struct%20Structure) (Ammount :type Integer))
  (Variables|Default|SetMap%20Key MapKey)
  (Variables|Default|SetAmmount Ammount))

(fn IsValidRecipe
  (params (In%20Item :type Name))
  (bind (_initemname _outitemname) (Utilities|LoopThroughDataTableRows)
    (:then
      (if (== _initemname In%20Item)
        (return (== _initemname In%20Item) _outitemname)))
    (:Completed
      (return false "None"))))