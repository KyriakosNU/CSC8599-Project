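; BP_RoundSystem tracks day and week numbers and refreshes player resources as each round begins.
; DayStart increments the day, triggers WeekStart on multiples of DaysPerWeek, then adds daily currency, sets time left and hunger, and prints the resources.
; WeekStart increments the week and resets environmental friendliness.
; PlayerResources is supplied through a setter, while DayEnd and WeekEnd are empty stubs.
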(event Custom|DayStart
  (bind _playerresources (Variables|Default|GetPlayerResources))
  ;[1 1 1 0.25] Day Events
  (bind _result (Math|Integer|IncrementInt (Variables|DayVariables|GetDayNo))
    (:%20%20
      (|IfIsStartOfWeek _result
        (:true
          (CallFunction|WeekStart))
        (:false
          _))
      (Utilities|IsValid _playerresources
        (:Is%20Valid
          (Default|AddtoCurrency _playerresources (Variables|DayVariables|PerDayConsts|GetCurrencyPerDay))
          (Default|SetTimeLeft _playerresources (Variables|DayVariables|PerDayConsts|GetTimePerDay))
          (Default|SetHunger _playerresources (Variables|DayVariables|PerDayConsts|GetHungerPerDay))
          (Default|PrintPlayerResources _playerresources 1e+01))))))

(event Custom|WeekStart
  (bind _playerresources (Variables|Default|GetPlayerResources))
  ;[1 1 1 0.25] Week Events
  (Math|Integer|IncrementInt (Variables|WeekVariables|GetWeekNo)
    (:%20%20
      (Utilities|IsValid _playerresources
        (:Is%20Valid
          (Default|SetEnviromentalFriendliness _playerresources 1e+02))))))

(event Custom|DayEnd
  ;[1 1 1 0.25] Day Events
)

(event Custom|WeekEnd
  ;[1 1 1 0.25] Week Events
)

(fn SetPlayerResources
  (params (PlayerResources :type BP%20Player%20Resources%20Object%20Reference%20%28by%20ref%29))
  (Variables|Default|SetPlayerResources PlayerResources))