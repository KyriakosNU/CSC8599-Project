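; Cooler inventory that rescales the expiry of items by a CoolingFactor while they are stored in it.
; Adding items multiplies DaysToExpire by the factor, floors it, then calls the parent add.
; Transferring out asks the other inventory how many it can hold, adds that amount with expiry divided by the factor and floored, then removes the same amount under the original key.
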(fn AddItem(S)toInventory
  (params (Key :type F%20Inventory%20Map%20Key%20Struct%20Structure) (Ammount :type Integer))
  (bind _structout (Utilities|Struct|SetmembersinFInventoryMapKeyStruct Key (Math|Float|Floor (* (Utilities|Struct|BreakFInventoryMapKeyStruct Key) (Variables|Default|GetCoolingFactor)))))
  (|CallParentFunction _structout Ammount))

(fn TransferItem(s)toOtherInventory
  (params (Key :type F%20Inventory%20Map%20Key%20Struct%20Structure%20%28by%20ref%29) (Ammount :type Integer))
  (bind _otherinventory (Variables|Default|GetOtherInventory))
  (Utilities|IsValid _otherinventory
    (:Is%20Valid
      (bind _returnvalue (Default|GetAmmountThatCanbeHeld _otherinventory Key Ammount))
      (if (> _returnvalue 0)
        (bind _structout (Utilities|Struct|SetmembersinFInventoryMapKeyStruct (|Copy Key) (Math|Float|Floor (/ (Utilities|Struct|BreakFInventoryMapKeyStruct Key) (Variables|Default|GetCoolingFactor)))))
        (CallFunction|AddItem(S)toInventory (Variables|Default|GetOtherInventory) _structout _returnvalue)
        (CallFunction|RemoveItem(s)fromInventory Key _returnvalue)
        (return)))))